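; Celestial body actor that holds mass, radius, material and starting velocity, with Niagara visuals for its orbit trail and gravity field.
; Radius drives actor scale, and mass sets three gravity-field rings through a clamped square root.
; On BeginPlay it records location and velocity, hides the field, and gives non-static bodies a random-colored trail.
; Helper functions control selection outline, field visibility and trail state; the actor contains no movement logic.
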(event EventBeginPlay
  (Variables|Default|SetInitialLocation (Transformation|GetActorLocation))
  (Variables|Default|SetVelocity (Variables|Default|GetInitialVelocity))
  (CallFunction|UpdateGravityField)
  (Rendering|SetVisibility (Variables|Default|GetNS_GravityField) false false)
  (if (Variables|Default|GetIsStatic)
    (Components|Activation|Deactivate (Variables|Default|GetOrbitaTrail))
    (else
      (Components|Activation|Activate (Variables|Default|GetOrbitaTrail) false)
      (CallFunction|GenerateRandomTrailColor))))

(event Collision|EventActorBeginOverlap
  (params (OtherActor :type Actor%20Object%20Reference)))

(event EventTick
  (params (DeltaSeconds :type Float%20%28single-precision%29)))

(fn ConstructionScript
  (bind _radius (Variables|Default|GetRadius))
  (bind _returnvalue (/ _radius 5e+01))
  (Transformation|SetActorScale3D (Math|Vector|MakeVector _returnvalue _returnvalue _returnvalue))
  (if (Utilities|IsValid (Variables|Default|GetBodyMaterial))
    (Rendering|Material|SetMaterial (Variables|Default|GetBodyMesh) 0 (Variables|Default|GetBodyMaterial))))

(fn SetSelectedVisual
  (params (IsSelected :type Boolean))
  (Rendering|SetVisibility (Variables|Default|GetSelectedOutlinerMesh) IsSelected true))

(fn ApplyRadiusScale
  (bind _radius (Variables|Default|GetRadius))
  (bind _returnvalue (/ _radius 5e+01))
  (Transformation|SetActorScale3D (Math|Vector|MakeVector _returnvalue _returnvalue _returnvalue)))

(fn ApplyBodyMaterial
  (if (Utilities|IsValid (Variables|Default|GetBodyMaterial))
    (Rendering|Material|SetMaterial (Variables|Default|GetBodyMesh) 0 (Variables|Default|GetBodyMaterial))))

(fn ResetTrail
  (Niagara|ReinitializeSystem (Variables|Default|GetOrbitaTrail)))

(fn SetTrailPaused
  (params (Paused :type Boolean))
  (Class|NiagaraComponent|SetPaused (Variables|Default|GetOrbitaTrail) Paused))

(fn UpdateGravityField
  (LocalVariables|SetBaseFieldRadius (Math|Float|Clamp(Float) (* (Math|Float|Sqrt (Variables|Default|GetMass)) 5.0) 1e+02 8e+02))
  (LocalVariables|SetInnerRadius (* (LocalVariables|GetBaseFieldRadius) 0.33))
  (LocalVariables|SetMiddleRadius (* (LocalVariables|GetBaseFieldRadius) 0.66))
  (LocalVariables|SetOuterRadius (LocalVariables|GetBaseFieldRadius))
  (Niagara|SetNiagaraVariable(Float) (Variables|Default|GetNS_GravityField) "User.GravityRadius01" (LocalVariables|GetInnerRadius))
  (Niagara|SetNiagaraVariable(Float) (Variables|Default|GetNS_GravityField) "User.GravityRadius02" (LocalVariables|GetMiddleRadius))
  (Niagara|SetNiagaraVariable(Float) (Variables|Default|GetNS_GravityField) "User.GravityRadius03" (LocalVariables|GetOuterRadius))
  (Niagara|ReinitializeSystem (Variables|Default|GetNS_GravityField)))

(fn SetGravityFieldVisible
  (params (Visible :type Boolean))
  (Rendering|SetVisibility (Variables|Default|GetNS_GravityField) Visible false))

(fn GenerateRandomTrailColor
  (Variables|Default|SetTrailColor (Utilities|Struct|MakeLinearColor (Math|Random|RandomFloatinRange 0.4 0.5) (Math|Random|RandomFloatinRange 0.4 1.0) (Math|Random|RandomFloatinRange 0.4 1.0) 1.0))
  (CallFunction|UpdateTrailColor))

(fn UpdateTrailColor
  (Niagara|SetNiagaraVariable(LinearColor) (Variables|Default|GetOrbitaTrail) "User.TrailColor" (Variables|Default|GetTrailColor))
  (Niagara|ReinitializeSystem (Variables|Default|GetOrbitaTrail)))