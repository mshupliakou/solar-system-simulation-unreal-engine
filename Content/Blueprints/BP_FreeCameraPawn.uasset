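; Free-flying camera pawn for a solar system scene that lets the player move around and click celestial bodies to select them.
; Axis inputs drive movement along the actor's forward, right and up vectors, and feed controller yaw and pitch for looking.
; Left click runs a complex Visibility trace under the cursor and passes any hit BP_CelestialBody to the BP_SolarSystemManager cached at BeginPlay.
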(event EventBeginPlay
  (bind _outactors (Actor|GetAllActorsOfClass "/Game/Blueprints/BP_SolarSystemManager.BP_SolarSystemManager_C"))
  (Variables|Default|SetManagerRef (Utilities|Array|Get(acopy) _outactors)))

(event Collision|EventActorBeginOverlap
  (params (OtherActor :type Actor%20Object%20Reference)))

(event EventTick
  (params (DeltaSeconds :type Float%20%28single-precision%29)))

(event Input|AxisEvents|InputAxisMoveForward
  (params (AxisValue :type Float%20%28single-precision%29))
  ;[0.15 0.06258 0.06516 0.5] Ruch do przodu/tylu
  (Pawn|Input|AddMovementInput (Transformation|GetActorForwardVector) AxisValue false))

(event Input|AxisEvents|InputAxisMoveRight
  (params (AxisValue :type Float%20%28single-precision%29))
  ;[0.08541 0.06279 0.15 0.5] Ruch lewo/prawo
  (Pawn|Input|AddMovementInput (Transformation|GetActorRightVector) AxisValue false))

(event Input|AxisEvents|InputAxisMoveUp
  (params (AxisValue :type Float%20%28single-precision%29))
  ;[0.15 0.15 0.15 0.5] Ruch gora/dol
  (Pawn|Input|AddMovementInput (Transformation|GetActorUpVector) AxisValue false))

(event Input|AxisEvents|InputAxisTurn
  (params (AxisValue :type Float%20%28single-precision%29))
  ;[0.08625 0.1242 0.15 0.5] Obrot muszka
  (Pawn|Input|AddControllerYawInput AxisValue))

(event Input|AxisEvents|InputAxisLookUp
  (params (AxisValue :type Float%20%28single-precision%29))
  ;[0.08625 0.1242 0.15 0.5] Obrot muszka
  (Pawn|Input|AddControllerPitchInput AxisValue))

(event Input|MouseEvents|LeftMouseButton
  (params (Key :type Key%20Structure :default "None"))
  (bind _returnvalue (Game|GetPlayerController 0))
  (bind (_hitresult _returnvalue_2) (Game|Player|GetHitResultUnderCursorbyChannel _returnvalue "TraceTypeQuery1" true))
  (:Pressed
    (if _returnvalue_2
      (bind _asbp_celestial_body (Utilities|Casting|CastToBP_CelestialBody (.HitActor (Collision|BreakHitResult _hitresult))))
      (Default|SetSelectedBody (Variables|Default|GetManagerRef) _asbp_celestial_body))))

(fn ConstructionScript)