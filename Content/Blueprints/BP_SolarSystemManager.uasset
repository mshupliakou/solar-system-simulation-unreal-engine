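; Manager actor that runs an N-body gravity simulation of all BP_CelestialBody actors in the level.
; Tick runs fixed-step velocity Verlet substeps with softened pairwise gravity, moving only non-static bodies; P pauses, R resets.
; BeginPlay gathers bodies, seeds accelerations and creates WBP_ControlPanel inside the per-body loop.
; Selection functions switch, edit mass or velocity, and delete bodies, recomputing accelerations after mass changes and deletions.
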(event EventBeginPlay
  (bind _outactors (Actor|GetAllActorsOfClass "/Game/Blueprints/BP_CelestialBody.BP_CelestialBody_C"))
  (bind _output_get (Variables|Default|SetBodies _outactors))
  (if (> (Utilities|Array|Length (Variables|Default|GetBodies)) 0)
    (bind _output_get_2 (Variables|Default|SetSelectedBody (Utilities|Array|Get(acopy) _output_get)))
    (Default|SetSelectedVisual _output_get_2 true)
    (for _array_element _output_get
      (bind _resultacceleration (CallFunction|CalculateAccelerationforBody _array_element))
      (Variables|/Game/Blueprints/BP_CelestialBody.BP_CelestialBody_C|SetAcceleration _array_element _resultacceleration)
      (bind _returnvalue (UserInterface|CreateWidget "/Game/UI/WBP_ControlPanel.WBP_ControlPanel_C"))
      (bind _output_get_3 (Variables|Default|SetControlPanelRef _returnvalue))
      (UserInterface|Viewport|AddtoViewport _returnvalue 0)
      (Variables|/Script/Engine.PlayerController|SetbShowMouseCursor (Game|GetPlayerController 0) true)
      (Input|SetInputModeGameandUI (Game|GetPlayerController 0) 0 "DoNotLock" true false))))

(event Collision|EventActorBeginOverlap
  (params (OtherActor :type Actor%20Object%20Reference)))

(event EventTick
  (params (DeltaSeconds :type Float%20%28single-precision%29))
  (if (not (Variables|Default|GetIsPaused))
    (for _index (range 0 (- (Variables|Default|GetSubstepsPerTick) 1))
      (CallFunction|SimulateStep (Variables|Default|GetFixedTimeStep)))))

(event Input|KeyboardEvents|P
  (params (Key :type Key%20Structure :default "None"))
  (:Pressed
    (Variables|Default|SetIsPaused (not (Variables|Default|GetIsPaused)))))

(event Input|KeyboardEvents|R
  (params (Key :type Key%20Structure :default "None"))
  (:Pressed
    (CallFunction|ResetSystem)))

(fn ConstructionScript)

(fn CalculateAccelerationforBody
  (params (TargetBody :type BP%20Celestial%20Body%20Object%20Reference))
  (LocalVariables|SetTargetBody_Local TargetBody)
  (LocalVariables|SetAccelerationSum "0, 0, 0")
  (for _array_element (Variables|Default|GetBodies)
    (LocalVariables|SetOtherBody _array_element)
    (if (!= (LocalVariables|GetTargetBody_Local) (LocalVariables|GetOtherBody))
      (LocalVariables|SetAccelerationSum (+ (/ (* (Math|Vector|Normalize (- (Transformation|GetActorLocation (LocalVariables|GetOtherBody)) (Transformation|GetActorLocation (LocalVariables|GetTargetBody_Local)))) (Variables|Default|GetGravityConstant) (Variables|/Game/Blueprints/BP_CelestialBody.BP_CelestialBody_C|GetMass (LocalVariables|GetOtherBody))) (+ (* (Variables|Default|GetSoftening) (Variables|Default|GetSoftening)) (Math|Vector|VectorLengthSquared (- (Transformation|GetActorLocation (LocalVariables|GetOtherBody)) (Transformation|GetActorLocation (LocalVariables|GetTargetBody_Local)))))) (LocalVariables|GetAccelerationSum)))))
  (return (LocalVariables|GetAccelerationSum)))

(fn SimulateStep
  (params (Dt :type Float%20%28double-precision%29))
  (LocalVariables|Setdelta Dt)
  ;[0.15 0.15 0.15 0.5] Faza 1: aktualizacja pozycji
  (for _array_element (Variables|Default|GetBodies)
    (LocalVariables|SetBody_fase1 _array_element)
    (if (not (Variables|/Game/Blueprints/BP_CelestialBody.BP_CelestialBody_C|GetIsStatic _array_element))
      (Variables|/Game/Blueprints/BP_CelestialBody.BP_CelestialBody_C|SetPreviousAcceleration (LocalVariables|GetBody_fase1) (Variables|/Game/Blueprints/BP_CelestialBody.BP_CelestialBody_C|GetAcceleration (LocalVariables|GetBody_fase1)))
      (Transformation|SetActorLocation (LocalVariables|GetBody_fase1) (+ (Transformation|GetActorLocation (LocalVariables|GetBody_fase1)) (* (Variables|/Game/Blueprints/BP_CelestialBody.BP_CelestialBody_C|GetVelocity (LocalVariables|GetBody_fase1)) (LocalVariables|Getdelta)) (* (Variables|/Game/Blueprints/BP_CelestialBody.BP_CelestialBody_C|GetAcceleration (LocalVariables|GetBody_fase1)) 0.5 (LocalVariables|Getdelta) (LocalVariables|Getdelta))) false false)))
  ;[0.1153 0.15 0.08837 0.5] Faza 2: przeliczenie nowego przyspieszenia
  (for _array_element_2 (Variables|Default|GetBodies)
    (bind _resultacceleration (CallFunction|CalculateAccelerationforBody _array_element_2))
    (Variables|/Game/Blueprints/BP_CelestialBody.BP_CelestialBody_C|SetAcceleration _array_element_2 _resultacceleration))
  ;[0.06502 0.06824 0.15 0.5] Faza 3: aktualizacja prędkości
  (for _array_element_3 (Variables|Default|GetBodies)
    (LocalVariables|SetBody_fase3 _array_element_3)
    (if (not (Variables|/Game/Blueprints/BP_CelestialBody.BP_CelestialBody_C|GetIsStatic _array_element_3))
      (Variables|/Game/Blueprints/BP_CelestialBody.BP_CelestialBody_C|SetVelocity (LocalVariables|GetBody_fase3) (+ (Variables|/Game/Blueprints/BP_CelestialBody.BP_CelestialBody_C|GetVelocity (LocalVariables|GetBody_fase3)) (* (+ (Variables|/Game/Blueprints/BP_CelestialBody.BP_CelestialBody_C|GetPreviousAcceleration (LocalVariables|GetBody_fase3)) (Variables|/Game/Blueprints/BP_CelestialBody.BP_CelestialBody_C|GetAcceleration (LocalVariables|GetBody_fase3))) 0.5 (LocalVariables|Getdelta)))))))

(fn ResetSystem
  (for _array_element (Variables|Default|GetBodies)
    (bind _output_get (LocalVariables|SetCurrentBody _array_element))
    (Transformation|SetActorLocation _output_get (Variables|/Game/Blueprints/BP_CelestialBody.BP_CelestialBody_C|GetInitialLocation _array_element) false false)
    (Variables|/Game/Blueprints/BP_CelestialBody.BP_CelestialBody_C|SetVelocity (LocalVariables|GetCurrentBody) (Variables|/Game/Blueprints/BP_CelestialBody.BP_CelestialBody_C|GetInitialVelocity (LocalVariables|GetCurrentBody)))
    (Variables|/Game/Blueprints/BP_CelestialBody.BP_CelestialBody_C|SetAcceleration (LocalVariables|GetCurrentBody) "0, 0, 0")
    (Variables|/Game/Blueprints/BP_CelestialBody.BP_CelestialBody_C|SetPreviousAcceleration (LocalVariables|GetCurrentBody) "0, 0, 0")))

(fn RecalculateAllAccelerations
  (for _array_element (Variables|Default|GetBodies)
    (bind _resultacceleration (CallFunction|CalculateAccelerationforBody _array_element))
    (Variables|/Game/Blueprints/BP_CelestialBody.BP_CelestialBody_C|SetAcceleration _array_element _resultacceleration)))

(fn SelectNextBody
  (Variables|Default|SetSelectedIndex (+ (Variables|Default|GetSelectedIndex) 1))
  (if (>= (Variables|Default|GetSelectedIndex) (Utilities|Array|Length (Variables|Default|GetBodies)))
    (Variables|Default|SetSelectedIndex 0))
  (bind _output_get (Variables|Default|SetSelectedBody (Utilities|Array|Get(acopy) (Variables|Default|GetBodies) (Variables|Default|GetSelectedIndex))))
  (Development|PrintString (Utilities|GetDisplayName _output_get)))

(fn ApplyMasstoSelected
  (params (NewMass :type Float%20%28double-precision%29))
  (if (Utilities|IsValid (Variables|Default|GetSelectedBody))
    (Variables|/Game/Blueprints/BP_CelestialBody.BP_CelestialBody_C|SetMass (Variables|Default|GetSelectedBody) NewMass)
    (CallFunction|RecalculateAllAccelerations)))

(fn ApplyVelocitytoSelected
  (params (NewVelocity :type Vector))
  (if (Utilities|IsValid (Variables|Default|GetSelectedBody))
    (if (Variables|/Game/Blueprints/BP_CelestialBody.BP_CelestialBody_C|GetIsStatic (Variables|Default|GetSelectedBody))
      (Development|PrintString "Cannot change velocity at static body")
      (else
        (bind _output_get (Variables|/Game/Blueprints/BP_CelestialBody.BP_CelestialBody_C|SetVelocity (Variables|Default|GetSelectedBody) NewVelocity))
        (Variables|/Game/Blueprints/BP_CelestialBody.BP_CelestialBody_C|SetInitialVelocity (Variables|Default|GetSelectedBody) _output_get)))))

(fn DeleteSelectedBody
  (if (Utilities|IsValid (Variables|Default|GetSelectedBody))
    (if (Variables|/Game/Blueprints/BP_CelestialBody.BP_CelestialBody_C|GetIsStatic (Variables|Default|GetSelectedBody))
      (Development|PrintString "Cannot delete static body")
      (else
        (Utilities|Array|RemoveItem (Variables|Default|GetBodies) (Variables|Default|GetSelectedBody))
        (Default|SetSelectedVisual (Variables|Default|GetSelectedBody) false)
        (Actor|DestroyActor (Variables|Default|GetSelectedBody))
        (if (> (Utilities|Array|Length (Variables|Default|GetBodies)) 0)
          (Variables|Default|SetSelectedIndex 0)
          (bind _output_get (Variables|Default|SetSelectedBody (Utilities|Array|Get(acopy) (Variables|Default|GetBodies) (Variables|Default|GetSelectedIndex))))
          (Default|SetSelectedVisual _output_get true)
          (else
            (Variables|Default|SetSelectedBody 0)))
        (CallFunction|RecalculateAllAccelerations)))))

(fn SetSelectedBody
  (params (NewSelectedBody :type BP%20Celestial%20Body%20Object%20Reference))
  (if (Utilities|IsValid (Variables|Default|GetSelectedBody))
    (Default|SetSelectedVisual (Variables|Default|GetSelectedBody) false)
    (Variables|Default|SetSelectedBody NewSelectedBody)
    (if (Utilities|IsValid (Variables|Default|GetSelectedBody))
      (Default|SetSelectedVisual (Variables|Default|GetSelectedBody) true)
      (if (Utilities|IsValid (Variables|Default|GetControlPanelRef))
        (Default|RefreshSelectedBodyValues (Variables|Default|GetControlPanelRef))
        (Development|PrintString (Utilities|GetDisplayName (Variables|Default|GetSelectedBody)))))))